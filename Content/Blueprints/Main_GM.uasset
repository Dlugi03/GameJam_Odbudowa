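; Game mode that runs the HUD and end-of-game screens for a coin-driven, staged tower objective.
; BeginPlay finds the TowerManager, creates the HUD and starts a gameplay timer; Tick polls the manager to refresh coin and stage text.
; On WinGame, Tick swaps in the win screen, UI-only input and tower cinematic, with no once-only guard.
; A matching lose branch exists but is unreachable behind a constant condition.
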(event EventBeginPlay
  (Variables|Default|SetGameplayTime (* -1 (Class|GameplayStatics|GetUnpausedTimeSeconds)))
  (bind _outactors (Actor|GetAllActorsOfClass "/Script/GameJam_Odbudowa.TowerManager_Actor"))
  (Variables|Default|SetTowerManager (Utilities|Array|Get(acopy) _outactors))
  (bind _returnvalue (UserInterface|CreateWidget "/Game/UI/HUD/MainHUD.MainHUD_C" (Game|GetPlayerController 0)))
  (bind _output_get (Variables|Default|SetMainHUD_Ref _returnvalue))
  (UserInterface|Viewport|AddtoViewport _output_get 0)
  (bind _asplayer_char_2 (Utilities|Casting|CastToPlayer_char2 (Game|GetPlayerCharacter 0)))
  (Variables|Default|SetPlayer_Ref _asplayer_char_2))

(event EventTick
  (params (DeltaSeconds :type Float%20%28single-precision%29))
  (bind _returnvalue (Game|GetPlayerController 0))
  (bind _returnvalue_2 (Game|GetPlayerController 0))
  (bind _towermanager (Variables|Default|GetTowerManager))
  (bind _towermanager_2 (Variables|Default|GetTowerManager))
  (bind _mainhud_ref (Variables|Default|GetMainHUD_Ref))
  (bind _mainhud_ref_2 (Variables|Default|GetMainHUD_Ref))
  (if (not false)
    (Utilities|IsValid _towermanager
      (:Is%20Valid
        (if (Variables|/Script/GameJam_Odbudowa.TowerManager_Actor|GetbWinGame _towermanager)
          (Variables|Default|SetGameplayTime (+ (Variables|Default|GetGameplayTime) (Class|GameplayStatics|GetUnpausedTimeSeconds)))
          (Widget|RemovefromParent (Variables|Default|GetMainHUD_Ref))
          (bind _returnvalue_3 (UserInterface|CreateWidget "/Game/UI/WinGame/WinGame__W.WinGame__W_C" _returnvalue_2))
          (UserInterface|Viewport|AddtoViewport _returnvalue_3 0)
          (Variables|/Script/Engine.PlayerController|SetbShowMouseCursor _returnvalue_2 true)
          (Input|SetInputModeUIOnly _returnvalue_2 0 "DoNotLock")
          (Sequencer|Player|CreateLevelSequencePlayer "/Game/PACMAN/CINEMATIC/WIEŻACINEMATIC.WIEŻACINEMATIC" (Utilities|Struct|MakeMovieSceneSequencePlaybackSettings true "(Value=0)" 1.0 0.0 false false true false false false false true))
          (else
            (Variables|/Game/UI/HUD/MainHUD.MainHUD_C|SetCoinsAtStage _mainhud_ref_2 (Utilities|Array|Get(acopy) (Variables|/Script/GameJam_Odbudowa.TowerManager_Actor|GetCoinsForNextStage _towermanager_2) (Variables|/Script/GameJam_Odbudowa.TowerManager_Actor|GetCurrentStage _towermanager_2)))
            (Variables|/Game/UI/HUD/MainHUD.MainHUD_C|SetCollectedCoinsAtStage _mainhud_ref_2 (Variables|/Script/GameJam_Odbudowa.TowerManager_Actor|GetCoinsAtStage (Variables|Default|GetTowerManager)))
            (Default|UpdateCoinsText _mainhud_ref_2)
            (Variables|/Game/UI/HUD/MainHUD.MainHUD_C|SetStageIndex _mainhud_ref (Variables|/Script/GameJam_Odbudowa.TowerManager_Actor|GetCurrentStage (Variables|Default|GetTowerManager)))
            (Default|UpdateStageText _mainhud_ref)))))
    (else
      (Widget|RemovefromParent (Variables|Default|GetMainHUD_Ref))
      (bind _returnvalue_4 (UserInterface|CreateWidget "/Game/UI/WinGame/LoseGame_W.LoseGame_W_C" _returnvalue))
      (UserInterface|Viewport|AddtoViewport _returnvalue_4 0)
      (Variables|/Script/Engine.PlayerController|SetbShowMouseCursor _returnvalue true)
      (Input|SetInputModeUIOnly _returnvalue 0 "DoNotLock")
      (Sequencer|Player|CreateLevelSequencePlayer "/Game/PACMAN/CINEMATIC/WIEŻACINEMATIC.WIEŻACINEMATIC" (Utilities|Struct|MakeMovieSceneSequencePlaybackSettings true "(Value=0)" 1.0 0.0 false false true false false false false true)))))

(fn ConstructionScript)